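; AI controller for the patrolling guard NPC that reacts to perceived targets by aiming and shooting.
; On BeginPlay it sets up the PatrolData blackboard and runs the GuardBehavior behavior tree.
; AI Perception updates for actors without the "Enemy" tag set or clear the blackboard enemy key as they are sensed or lost.
; The same updates toggle the aiming and shooting flags on the controlled TPCharacter_BP pawn.
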(event OnTargetPerceptionUpdated(AIPerception)
  (params (Actor :type Actor%20Object%20Reference) (Stimulus :type AI%20Stimulus%20Structure))
  (bind _returnvalue (Pawn|GetControlledPawn))
  (if (not (Actor|ActorHasTag Actor "Enemy"))
    (if (.bSuccessfullySensed (Utilities|Struct|BreakAIStimulus Stimulus))
      (AI|Components|Blackboard|SetValueasObject (Variables|Default|GetBlackBoardComp) (Variables|Default|GetEnemyKey) Actor)
      (bind _astpcharacter_bp (Utilities|Casting|CastToTPCharacter_BP _returnvalue))
      (Variables|/Game/Dynamic/NPC/PatrollingGuard/Behavior/TPCharacter_BP.TPCharacter_BP_C|SetAiming%20at%20target _astpcharacter_bp true)
      (Variables|/Game/Dynamic/NPC/PatrollingGuard/Behavior/TPCharacter_BP.TPCharacter_BP_C|SetShooting%20at%20target _astpcharacter_bp true)
      (else
        (AI|Components|Blackboard|ClearValue (Variables|Default|GetBlackBoardComp) (Variables|Default|GetEnemyKey))
        (bind _astpcharacter_bp_2 (Utilities|Casting|CastToTPCharacter_BP _returnvalue))
        (Variables|/Game/Dynamic/NPC/PatrollingGuard/Behavior/TPCharacter_BP.TPCharacter_BP_C|SetAiming%20at%20target _astpcharacter_bp_2 false)
        (Variables|/Game/Dynamic/NPC/PatrollingGuard/Behavior/TPCharacter_BP.TPCharacter_BP_C|SetShooting%20at%20target _astpcharacter_bp_2 false)))))

(event EventBeginPlay
  (bind _blackboardcomponent (Class|AIController|UseBlackboard "/Game/Dynamic/NPC/PatrollingGuard/AI/PatrolData.PatrolData"))
  (Variables|Default|SetBlackBoardComp _blackboardcomponent)
  (AI|RunBehaviorTree "/Game/Dynamic/NPC/PatrollingGuard/AI/GuardBehavior.GuardBehavior"))

(fn ConstructionScript)