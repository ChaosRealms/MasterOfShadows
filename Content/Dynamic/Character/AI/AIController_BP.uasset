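; AI controller for guard characters that runs the GuardBehavior tree on a PatrolData blackboard and tracks a detected player.
; Perception updates set the blackboard enemy key to a living, sensed Character_BP not tagged Enemy.
; The key clears when that character dies or a perception update reports it lost.
; Acquiring a target while the key is empty also notifies InfiniteTerrainGameMode that the player was detected.
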(event OnTargetPerceptionUpdated(AIPerception)
  (params (Actor :type Actor%20Object%20Reference) (Stimulus :type AI%20Stimulus%20Structure))
  (CallFunction|UpdateBlackBoardEnemyKey Stimulus Actor))

(event EventBeginPlay
  (bind _blackboardcomponent (Class|AIController|UseBlackboard "/Game/Dynamic/Character/AI/PatrolData.PatrolData"))
  (Variables|Default|SetBlackBoardComp _blackboardcomponent)
  (AI|RunBehaviorTree "/Game/Dynamic/Character/AI/GuardBehavior.GuardBehavior"))

(fn ConstructionScript)

(fn UpdateBlackBoardEnemyKey
  (params (AIStimulus :type AI%20Stimulus%20Structure%20%28by%20ref%29) (PlayerActor :type Actor%20Object%20Reference))
  (bind _ascharacter_bp (Utilities|Casting|CastToCharacter_BP PlayerActor))
  (if (Default|IsDead _ascharacter_bp)
    (CallFunction|ClearEnemyKey)
    (elif (not (Actor|ActorHasTag PlayerActor "Enemy"))
      (if (.bSuccessfullySensed (Utilities|Struct|BreakAIStimulus AIStimulus))
        (CallFunction|SetEnemyDetected PlayerActor)
        (else
          (CallFunction|ClearEnemyKey))))))

(fn ClearEnemyKey
  (AI|Components|Blackboard|ClearValue (Variables|Default|GetBlackBoardComp) (Variables|Default|GetEnemyKey)))

(fn SetEnemyDetected
  (params (PlayerObject :type Object%20Object%20Reference))
  (Utilities|IsValid (AI|Components|Blackboard|GetValueasObject (Variables|Default|GetBlackBoardComp) (Variables|Default|GetEnemyKey))
    (:Is%20Not%20Valid
      (AI|Components|Blackboard|SetValueasObject (Variables|Default|GetBlackBoardComp) (Variables|Default|GetEnemyKey) PlayerObject)
      (CallFunction|OnPlayerDetected))))

(fn OnPlayerDetected
  (bind _returnvalue (Game|GetGameMode))
  (Utilities|IsValid _returnvalue
    (:Is%20Valid
      (bind _asinfinite_terrain_game_mode (Utilities|Casting|CastToInfiniteTerrainGameMode _returnvalue))
      (Default|CallOnPlayerDetected _asinfinite_terrain_game_mode))))