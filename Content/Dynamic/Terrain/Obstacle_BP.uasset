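; Obstacle Blueprint that gives each spawned terrain obstacle a random size and color.
; On BeginPlay it scales its static mesh independently on each axis within a random range.
; It then creates a dynamic instance of the LevelBasic material, sets a random color and alpha through a vector parameter, and applies it to the mesh.
; The construction script is empty, so all variation happens at runtime.
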(event EventBeginPlay
  (bind _returnvalue (Math|Random|RandomFloatinRange 2.0 5.0))
  (Transformation|SetRelativeScale3D (Variables|Default|GetStaticMesh) (Math|Vector|MakeVector _returnvalue _returnvalue _returnvalue))
  (bind _returnvalue_2 (Rendering|Material|CreateDynamicMaterialInstance (Variables|Default|GetStaticMesh) 0 "/Game/Dynamic/Terrain/LevelBasic.LevelBasic" :!class /Script/Engine.PrimitiveComponent))
  (Rendering|Material|SetVectorParameterValue _returnvalue_2 "VectorParamBasic" (Utilities|Struct|MakeLinearColor (Math|Random|RandomFloat) (Math|Random|RandomFloat) (Math|Random|RandomFloat) (Math|Random|RandomFloatinRange 0.5 1.0)) :!class /Script/Engine.MaterialInstanceDynamic)
  (Rendering|Material|SetMaterial (Variables|Default|GetStaticMesh) 0 _returnvalue_2))

(fn ConstructionScript)